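; VR player character Blueprint that handles headset startup when play begins.
; If a head-mounted display is enabled, BeginPlay sets a local-floor tracking origin, sets the secondary screen percentage by console command, then hides the loading screen.
; Logic for spawning and attaching left and right hand actors and adding default and hand input mapping contexts is present but disconnected, so it never runs.
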(event EventBeginPlay
  (Utilities|FlowControl|Sequence
    (:then_0
      (if (Class|HeadMountedDisplayFunctionLibrary|IsHeadMountedDisplayEnabled)
        (Utilities|FlowControl|Sequence
          (:then_0
            (Class|HeadMountedDisplayFunctionLibrary|SetTrackingOrigin "LocalFloor")
            (Development|ExecuteConsoleCommand "xr.SecondaryScreenPercentage.HMDRenderTarget 100" 0))
          (:then_1
            (Class|XRLoadingScreenFunctionLibrary|HideLoadingScreen) ; See WidgetMenu for loading screen logic
          ))))))

(event Collision|EventActorBeginOverlap
  (params (OtherActor :type Actor%20Object%20Reference)))

(event EventTick
  (params (DeltaSeconds :type Float%20%28single-precision%29)))

(fn ConstructionScript)