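; Left VR hand Blueprint that poses its hand mesh from the player's left-hand Enhanced Input actions.
; Each action writes a pose alpha on the mesh's ABP_MannequinsXR anim instance.
; Grasp and index curl follow the action value and reset when completed or canceled.
; Point and thumb-up are inverted binary poses: cleared when input starts or cancels, fully applied when it completes.
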(event Input|EnhancedActionEvents|EnhancedInputActionIA_Hand_Grasp_Left
  (params (ActionValue :type Float%20%28double-precision%29) (ElapsedSeconds :type Float%20%28double-precision%29) (TriggeredSeconds :type Float%20%28double-precision%29) (InputAction :type Input%20Action%20Object%20Reference :default "/Game/XRFramework/Input/Actions/Hands/IA_Hand_Grasp_Left.IA_Hand_Grasp_Left"))
  (bind _handmesh (Variables|Default|GetHandMesh))
  (bind _returnvalue (Components|SkeletalMesh|GetAnimInstance _handmesh))
  (:Triggered
    (bind _asabp_mannequins_xr (Utilities|Casting|CastToABP_MannequinsXR _returnvalue))
    (Variables|/Game/XRMannequins/Meshes/ABP_MannequinsXR.ABP_MannequinsXR_C|SetPoseAlphaGrasp _asabp_mannequins_xr ActionValue))
  (:Canceled
    (bind _asabp_mannequins_xr_2 (Utilities|Casting|CastToABP_MannequinsXR _returnvalue :!label _label))
    (Variables|/Game/XRMannequins/Meshes/ABP_MannequinsXR.ABP_MannequinsXR_C|SetPoseAlphaGrasp _asabp_mannequins_xr_2 0.0))
  (:Completed
    (goto _label)))

(event Input|EnhancedActionEvents|EnhancedInputActionIA_Hand_Point_Left
  (params (ActionValue :type Float%20%28double-precision%29) (ElapsedSeconds :type Float%20%28double-precision%29) (TriggeredSeconds :type Float%20%28double-precision%29) (InputAction :type Input%20Action%20Object%20Reference :default "/Game/XRFramework/Input/Actions/Hands/IA_Hand_Point_Left.IA_Hand_Point_Left"))
  (bind _handmesh (Variables|Default|GetHandMesh))
  (:Started
    (bind _asabp_mannequins_xr (Utilities|Casting|CastToABP_MannequinsXR (Components|SkeletalMesh|GetAnimInstance _handmesh) :!label _label))
    (Variables|/Game/XRMannequins/Meshes/ABP_MannequinsXR.ABP_MannequinsXR_C|SetPoseAlphaPoint _asabp_mannequins_xr 0.0))
  (:Canceled
    (goto _label))
  (:Completed
    (bind _asabp_mannequins_xr_2 (Utilities|Casting|CastToABP_MannequinsXR (Components|SkeletalMesh|GetAnimInstance _handmesh)))
    (Variables|/Game/XRMannequins/Meshes/ABP_MannequinsXR.ABP_MannequinsXR_C|SetPoseAlphaPoint _asabp_mannequins_xr_2 1.0)))

(event Input|EnhancedActionEvents|EnhancedInputActionIA_Hand_ThumbUp_Left
  (params (ActionValue :type Float%20%28double-precision%29) (ElapsedSeconds :type Float%20%28double-precision%29) (TriggeredSeconds :type Float%20%28double-precision%29) (InputAction :type Input%20Action%20Object%20Reference :default "/Game/XRFramework/Input/Actions/Hands/IA_Hand_ThumbUp_Left.IA_Hand_ThumbUp_Left"))
  (bind _handmesh (Variables|Default|GetHandMesh))
  (:Started
    (bind _asabp_mannequins_xr (Utilities|Casting|CastToABP_MannequinsXR (Components|SkeletalMesh|GetAnimInstance _handmesh) :!label _label))
    (Variables|/Game/XRMannequins/Meshes/ABP_MannequinsXR.ABP_MannequinsXR_C|SetPoseAlphaThumbUp _asabp_mannequins_xr 0.0))
  (:Canceled
    (goto _label))
  (:Completed
    (bind _asabp_mannequins_xr_2 (Utilities|Casting|CastToABP_MannequinsXR (Components|SkeletalMesh|GetAnimInstance _handmesh)))
    (Variables|/Game/XRMannequins/Meshes/ABP_MannequinsXR.ABP_MannequinsXR_C|SetPoseAlphaThumbUp _asabp_mannequins_xr_2 1.0)))

(event Input|EnhancedActionEvents|EnhancedInputActionIA_Hand_IndexCurl_Left
  (params (ActionValue :type Float%20%28double-precision%29) (ElapsedSeconds :type Float%20%28double-precision%29) (TriggeredSeconds :type Float%20%28double-precision%29) (InputAction :type Input%20Action%20Object%20Reference :default "/Game/XRFramework/Input/Actions/Hands/IA_Hand_IndexCurl_Left.IA_Hand_IndexCurl_Left"))
  (bind _handmesh (Variables|Default|GetHandMesh))
  (bind _returnvalue (Components|SkeletalMesh|GetAnimInstance _handmesh))
  (:Triggered
    (bind _asabp_mannequins_xr (Utilities|Casting|CastToABP_MannequinsXR _returnvalue))
    (Variables|/Game/XRMannequins/Meshes/ABP_MannequinsXR.ABP_MannequinsXR_C|SetPoseAlphaIndexCurl _asabp_mannequins_xr ActionValue))
  (:Canceled
    (bind _asabp_mannequins_xr_2 (Utilities|Casting|CastToABP_MannequinsXR _returnvalue :!label _label))
    (Variables|/Game/XRMannequins/Meshes/ABP_MannequinsXR.ABP_MannequinsXR_C|SetPoseAlphaIndexCurl _asabp_mannequins_xr_2 0.0))
  (:Completed
    (goto _label)))

(event EventBeginPlay
  (|CallParentFunction))

(event Collision|EventActorBeginOverlap
  (params (OtherActor :type Actor%20Object%20Reference)))

(event EventTick
  (params (DeltaSeconds :type Float%20%28single-precision%29)))

(fn ConstructionScript)